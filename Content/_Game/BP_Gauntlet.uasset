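; BP_Gauntlet is a time-shifting gauntlet that trails the owner's left hand with eased drift and faces along the camera rotation.
; While shifting, a looping timer line-traces from the camera and sends age messages to BPI_Age or BPI_AgeSnap actors.
; Only BPI_Age hits drain Charge and update the material glow.
; Ending a shift or running empty stops the timer, then a delayed Timeline refills Charge from its current level.
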(event `self.ReceiveTick`
  (params (DeltaSeconds :type "Float (single-precision)"))
  (bind _returnvalue (`self.GetTransform`))
  (bind _gauntlet_drift (`self.Gauntlet Drift`))
  (bind (_returnvalue_x _returnvalue_y _returnvalue_z) (`KismetMathLibrary.BreakVector` (- (`SceneComponent.K2_GetComponentLocation` (`/Game/FirstPerson/Blueprints/BP_FirstPersonCharacter.Left Hand` (`self.Owner_Reference`))) (`KismetMathLibrary.MakeVector` (.x (.location _returnvalue)) (.y (.location _returnvalue)) (.z (.location _returnvalue))))))
  (`self.K2_SetActorTransform` (`KismetMathLibrary.MakeTransform` (`KismetMathLibrary.MakeVector` (+ (/ _returnvalue_x _gauntlet_drift) (.x (.location _returnvalue))) (+ (/ _returnvalue_y _gauntlet_drift) (.y (.location _returnvalue))) (+ (/ _returnvalue_z _gauntlet_drift) (.z (.location _returnvalue)))) (`PlayerCameraManager.GetCameraRotation` (`GameplayStatics.GetPlayerCameraManager` 0)))))

(event `Recharge`
  (if (`self.Recharging`)
    (`TimelineComponent.SetNewTime` (`self.Timeline_0`) (`self.Charge`))
    (bind (_direction _charging) (`Timeline|Timeline_0`)
      (:`Update`
        (set `self.Charge` (`KismetMathLibrary.Lerp` 0.0 1.0 _charging))))))

(event `ChangeGlow`
  (`MeshComponent.SetScalarParameterValueOnMaterials` (`self.Gauntlet_no_fingers`) "Glow" (`self.Charge`)))

(event `EndAging`
  ;[1 1 1] Small delay and starts recharging
  (`KismetSystemLibrary.K2_ClearAndInvalidateTimerHandle` (`self.Aging`))
  (set `self.IsAging` false)
  (set `self.Recharging` true)
  (`KismetSystemLibrary.Delay` 1.5)
  (`self.Recharge`))

(event `StartShifting`
  (`KismetSystemLibrary.PrintString` "Hello")
  (set `self.Recharging` false)
  (`self.AgeTarget`)
  (set `self.IsAging` true)
  (bind _returnvalue (`KismetSystemLibrary.K2_SetTimerDelegate` (delegate `AgeTarget`) (`self.FireRate`) true))
  (set `self.Aging` _returnvalue))

(event `EndShifting`
  (`self.EndAging`))

(event `AgeTarget`
  (bind _returnvalue (`GameplayStatics.GetPlayerCameraManager` 0))
  (bind _returnvalue_2 (`PlayerCameraManager.GetCameraLocation` _returnvalue))
  (if (> (`self.Charge`) 0.0)
    (bind (_outhit _returnvalue_3) (`KismetSystemLibrary.LineTraceSingle` :`Start` _returnvalue_2 :`End` (+ (* (`KismetMathLibrary.GetForwardVector` (`PlayerCameraManager.GetCameraRotation` _returnvalue)) 3000.0) _returnvalue_2) :`TraceChannel` "TraceTypeQuery1" :`DrawDebugType` "Persistent"))
    ;[1 1 1] Checks if hit object can be affected by time
    (if _returnvalue_3
      (bind (_bblockinghit _binitialoverlap _time _distance _location _impactpoint _normal _impactnormal _physmat _hitactor) (`GameplayStatics.BreakHitResult` _outhit))
      (if (`KismetSystemLibrary.DoesImplementInterface` _hitactor "/Game/TimeGauntlet/BPI_Age.BPI_Age_C")
        (set `self.Charge` (- (`self.Charge`) 0.05))
        (message `/Game/TimeGauntlet/BPI_Age.AgeUp` _hitactor (`self.AgeUp?`))
        (`self.ChangeGlow`)
        (elif (`KismetSystemLibrary.DoesImplementInterface` _hitactor "/Game/TimeGauntlet/BPI_AgeSnap.BPI_AgeSnap_C")
          (message `/Game/TimeGauntlet/BPI_AgeSnap.SnapAge` _hitactor (`self.AgeUp?`)))))
    (else
      (`self.EndAging`))))

(fn `UserConstructionScript`)