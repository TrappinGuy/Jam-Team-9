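; Base enemy whose CurrentAge drives its movement speed, strength, damage taken and material opacity.
; AgeUp steps age up or down, refreshing these stats; older enemies slow down, although the initial SetSpeed formula rises with age.
; Reaching zero or MaxAge hides and destroys the enemy after Death.
; Hit scales damage by age, and lethal hits only call Death, which prints and spawns any ItemDrop.
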(event `self.ReceiveBeginPlay`
  (set `self.BaseSpeed` (`CharacterMovementComponent.MaxWalkSpeed` (`self.CharacterMovement`)))
  (`self.SetSpeed`)
  (`self.SetStrength`))

(event `UpdateAge`
  ;[1 1 1] Replace with interface event
)

(event `UpdateSpeed`
  ;[1 1 1] Changes enemy speed based on age
  (bind _output_get (set `CharacterMovementComponent.MaxWalkSpeed` (* (- 1.0 (- (/ (`self.Current Age`) (`self.Max Age`)) 0.5)) (`self.BaseSpeed`)) (`self.CharacterMovement`)))
  (`self.UpdateTexture`))

(event `/Game/TimeGauntlet/BPI_Age.AgeUp`
  (params (AgeUp :type Boolean))
  (bind _current_age (`self.Current Age`))
  (bind _current_age_2 (`self.Current Age`))
  (bind _current_age_3 (`self.Current Age`))
  ;[1 1 1] Changes age
  (if AgeUp
    (if (not (>= _current_age_3 80.0))
      (set `self.Current Age` (+ _current_age 2.0))
      (`self.UpdateSpeed` :!label _label)
      (if (or (== _current_age_2 0.0) (== _current_age_2 (`self.Max Age`)))
        (`self.Death`)
        (`SceneComponent.SetVisibility` (`self.Mesh`) false false)
        (`KismetSystemLibrary.Delay` 0.2)
        (`self.K2_DestroyActor`)))
    (elif (> _current_age_3 0.0)
      (set `self.Current Age` (- _current_age 2.0))
      (goto _label))))

(event `/Game/BPI_Damagable.Hit`
  (params (Damage :type "Float (double-precision)"))
  ;[1 1 1] Handles taking damage
  (bind _output_get (set `self.Health` (- (`self.Health`) (* Damage (+ (/ (`self.Current Age`) (`self.Max Age`)) 0.5)))))
  (`KismetSystemLibrary.PrintString` (`KismetStringLibrary.Conv_DoubleToString` _output_get))
  (if (<= _output_get 0.0)
    (`self.Death`)))

(event `Death`
  (`KismetSystemLibrary.PrintString` (`KismetStringLibrary.Concat_StrStr` (`KismetSystemLibrary.GetObjectName` self) "Is Dead"))
  ;[1 1 1] Drops items on death (doesnt do anything yet, Item drop always empty)
  (if (not (== (`self.ItemDrop`) null))
    (`|SpawnActorFromClass` (`self.ItemDrop`) (`self.GetTransform` self) "Undefined" "OverrideRootScale" null null)))

(event `UpdateTexture`
  (`MeshComponent.SetScalarParameterValueOnMaterials` (`self.Mesh`) "Opacity" (/ (`self.Current Age`) (`self.Max Age`)))
  (`self.SetStrength`))

(fn `SetSpeed`
  (set `CharacterMovementComponent.MaxWalkSpeed` (+ (* (/ (`self.Current Age`) (`self.Max Age`)) (`self.MaxSpeed`)) (`self.MinSpeed`)) (`self.CharacterMovement`))
  (`self.UpdateTexture`))

(fn `SetStrength`
  (set `self.Strength` (+ (* (/ (`self.Current Age`) (`self.Max Age`)) (`self.MaxStrength`)) (`self.MinStrength`))))

(fn `UserConstructionScript`)