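; BP_EnemyTest is a test enemy that wanders randomly on the navmesh from BeginPlay.
; MoveNPC picks a random reachable point around the actor's current location, runs AI Move To, then re-calls itself after a delay, forming an endless roam loop.
; A failed move prints a debug "Hello" and retries after a shorter delay.
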(event `self.ReceiveBeginPlay`
  (`parent.ReceiveBeginPlay`)
  (`self.MoveNPC`))

(event `MoveNPC`
  (bind _output_get (set `self.Random Location` (`NavigationSystemV1.K2_GetRandomReachablePointInRadius` (`self.K2_GetActorLocation`) 1000.0 null null)))
  (`|AIMoveTo` self _output_get null
    (:`then`
      (`KismetSystemLibrary.Delay` 3.0)
      (`self.MoveNPC`))
    (:`OnFail`
      (`KismetSystemLibrary.PrintString` "Hello")
      (`KismetSystemLibrary.Delay` 0.2)
      (`self.MoveNPC`))))

(fn `UserConstructionScript`
  (`parent.UserConstructionScript`))