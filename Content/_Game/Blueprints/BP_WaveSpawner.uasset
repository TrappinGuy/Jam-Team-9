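; BP_WaveSpawner spawns enemy waves on a score budget that grows every second from BeginPlay.
; A self-recalling WaveTick prints the score and randomly triggers SpawnAttempt, which compares a random EnemyWaves cost key against that budget.
; Each enemy spawns at a random point in a box derived from SpawnPoints, and a key is deducted per enemy.
; Random picks are uncached, so checked, spawned and deducted keys can differ.
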(event `self.ReceiveBeginPlay`
  (`self.WaveTick`))

(event `WaveTick`
  (set `self.WaveScore` (+ (`self.WaveScore`) (`self.WaveScoreIncrease`)))
  (`KismetSystemLibrary.Delay` 1.0)
  (`self.WaveTick`)
  (`KismetSystemLibrary.PrintString` (`KismetStringLibrary.Conv_IntToString` (`self.WaveScore`)))
  (if (== (`KismetMathLibrary.RandomInteger` 11) 0)
    (`self.SpawnAttempt`)))

(event `SpawnAttempt`
  (bind _spawnpoints (`self.SpawnPoints`))
  (bind (_output_min _output_max) (break `Box` (`|GetArrayItem` _spawnpoints (`KismetMathLibrary.RandomInteger` (`KismetArrayLibrary.Array_Length` _spawnpoints)))))
  ;[1 1 1] Spawns enemy waves
  ;;[1 1 1] Get an enemy wave to spawn
  (bind _keys (`BlueprintMapLibrary.Map_Keys` (`self.EnemyWaves`)))
  (bind _output (`|GetArrayItem` _keys (`KismetMathLibrary.RandomInteger` (`KismetArrayLibrary.Array_Length` _keys))))
  (if (<= _output (`self.WaveScore`))
    (for _array_element (break `/Game/_Game/Blueprints/Struct_Waves` (`BlueprintMapLibrary.Map_Find` (`self.EnemyWaves`) _output))
      (`|SpawnActorFromClass` _array_element (`KismetMathLibrary.MakeTransform` (`KismetMathLibrary.RandomPointInBoundingBox` _output_min (/ _output_max (2.0 2.0 2.0)))) "Undefined" "OverrideRootScale" null null)
      ;;[1 1 1] Update Wave Score
      (set `self.WaveScore` (- (`self.WaveScore`) _output)))))

(fn `UserConstructionScript`)