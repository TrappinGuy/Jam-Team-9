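; Base enemy character Blueprint with an age mechanic that trades movement speed against damage resistance.
; UpdateAge, also called at BeginPlay, clamps age between zero and MaxAge, then rescales walk speed from the cached base so older enemies move slower.
; Hit scales incoming damage up with age and calls Death at zero health.
; Death only prints a message, and the other custom events print debug values.
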(event `self.ReceiveBeginPlay`
  (set `self.BaseSpeed` (`CharacterMovementComponent.MaxWalkSpeed` (`self.CharacterMovement`)))
  (`self.UpdateAge` -5.0))

(event `UpdateAge`
  (params (AgeChange :type "Float (double-precision)"))
  (bind _returnvalue (+ AgeChange (`self.Current Age`)))
  ;[1 1 1] Replace with interface event
  (if (> (`self.Max Age`) _returnvalue)
    (if (< _returnvalue 0.0)
      (set `self.Current Age` 0.0)
      (else
        (bind _output_get (set `self.Current Age` _returnvalue))))
    (else
      (set `self.Current Age` (`self.Max Age`))))
  (`self.UpdateSpeed`)
  (`KismetSystemLibrary.PrintString` (`KismetStringLibrary.Conv_DoubleToString` _output_get)))

(event `UpdateSpeed`
  (bind _output_get (set `CharacterMovementComponent.MaxWalkSpeed` (* (- 1.0 (- (/ (`self.Current Age`) (`self.Max Age`)) 0.5)) (`self.BaseSpeed`)) (`self.CharacterMovement`)))
  (`KismetSystemLibrary.PrintString` (`KismetStringLibrary.Conv_DoubleToString` _output_get)))

(event `/Game/BPI_Damagable.Hit`
  (params (Damage :type "Float (double-precision)"))
  (bind _output_get (set `self.Health` (- (`self.Health`) (* Damage (+ (/ (`self.Current Age`) (`self.Max Age`)) 0.5)))))
  (`KismetSystemLibrary.PrintString` (`KismetStringLibrary.Conv_DoubleToString` _output_get))
  (if (<= _output_get 0.0)
    (`self.Death`)))

(event `Death`
  (`KismetSystemLibrary.PrintString` (`KismetStringLibrary.Concat_StrStr` (`KismetSystemLibrary.GetObjectName` self) "Is Dead")))

(fn `UserConstructionScript`)