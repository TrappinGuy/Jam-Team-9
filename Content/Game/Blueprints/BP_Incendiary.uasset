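; BP_Incendiary is a short-lived fire area actor that deals repeated damage to actors inside its radius.
; On BeginPlay it adds a Niagara effect, sets a brief lifespan and starts a self-restarting DamageTick loop.
; Each tick sends HitMessage to DamageRadius overlaps implementing BPI_Damagable, then waits on a Delay before repeating until the actor expires.
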(event `self.ReceiveBeginPlay`
  (`AddComponent|NODE_AddNiagaraComponent-1`)
  (`self.SetLifeSpan` 3.0)
  (`self.DamageTick`))

(event `DamageTick`
  ;[1 1 1] Checks overlapping actors
  (for _array_element (`PrimitiveComponent.GetOverlappingActors` (`self.DamageRadius`) null)
    ;[1 1 1] If can hit, deals damage, then restarts damage tick
    (if (`KismetSystemLibrary.DoesImplementInterface` _array_element "/Game/BPI_Damagable.BPI_Damagable_C")
      (message `/Game/BPI_Damagable.Hit` _array_element 0.1)))
  (`KismetSystemLibrary.Delay` 0.3)
  (`self.DamageTick`))

(fn `UserConstructionScript`)