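; Melee enemy Blueprint that chases the player and strikes at close range, driven by a Pursue, Attack, Linger state loop in AITick.
; Pursue re-paths every half second to a standoff point near the player camera.
; Attack sends HitMessage to a Player-tagged actor inside its sphere, then lingers two seconds.
; SetVisibility hides both cubes and sets IsDying, blocking damage; the sword-swing animation logic is disconnected.
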(event `self.ReceiveBeginPlay`
  (`parent.ReceiveBeginPlay`)
  (`self.AI Tick`))

(event `AI Tick`
  (bind _returnvalue_location (`KismetMathLibrary.BreakTransform` (`self.GetTransform`)))
  (bind _in_range_of_player (`self.In_range_of_player`))
  (bind (_returnvalue_x _returnvalue_y _returnvalue_z) (`KismetMathLibrary.BreakVector` (`PlayerCameraManager.GetCameraLocation` (`GameplayStatics.GetPlayerCameraManager` 0))))
  (bind (_returnvalue_x_2 _returnvalue_y_2 _returnvalue_z_2) (`KismetMathLibrary.BreakVector` (`KismetMathLibrary.GetDirectionUnitVector` (`KismetMathLibrary.MakeVector` _returnvalue_x _returnvalue_y _returnvalue_z) _returnvalue_location)))
  (switch `/Game/Game/Blueprints/Enemies/ENUM_Melee_States` (`self.Current_State`)
    (:`NewEnumerator0`
      (`|AIMoveTo` self (`KismetMathLibrary.MakeVector` (+ (* _returnvalue_x_2 _in_range_of_player) _returnvalue_x) (+ (* _returnvalue_y_2 _in_range_of_player) _returnvalue_y) (+ (* _returnvalue_z_2 _in_range_of_player) _returnvalue_z)) null 100.0 :!label _label
        (:`then`
          (`KismetSystemLibrary.Delay` 0.5)
          (if (`|EnumEquality` (`self.Current_State`) (enumliteral `/Game/Game/Blueprints/Enemies/ENUM_Melee_States` "NewEnumerator0"))
            (goto _label)))
        (:`OnSuccess`
          (set `self.Current_State` "NewEnumerator1")
          (`self.AI Tick`))))
    (:`NewEnumerator1`
      (`KismetSystemLibrary.PrintString` "Hello1")
      (`self.Trigger Attack`)
      (`KismetSystemLibrary.PrintString` "Hello2")
      (set `self.Current_State` "NewEnumerator2")
      (`self.AI Tick`))
    (:`NewEnumerator2`
      (`KismetSystemLibrary.Delay` 2.0)
      (set `self.Current_State` "NewEnumerator0")
      (`self.AI Tick`))))

(event `self.Trigger Attack`
  (if (not (`self.IsDying`))
    (`self.SetStrength`)
    (for _array_element (`PrimitiveComponent.GetOverlappingActors` (`self.Sphere`) null)
      (if (`self.ActorHasTag` _array_element "Player")
        (message `/Game/BPI_Damagable.Hit` _array_element (`self.Strength`))
        (break)))))

(fn `SetVisibility`
  (`SceneComponent.SetVisibility` (`self.Cube1`) false false)
  (`SceneComponent.SetVisibility` (`self.Cube`) false false)
  (set `self.IsDying` true))

(fn `UserConstructionScript`
  (`parent.UserConstructionScript`))