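; Base enemy character whose age can be stepped up or down, scaling its speed, strength and damage resistance.
; Each age step recalculates movement speed, which falls with age, and strength, which rises, and sets the cube material's opacity from age.
; Reaching zero or max age kills and destroys it, while lethal hits only call Death, which spawns any set item drop.
; Freeze only prints and TriggerAttack is empty.
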(event `self.ReceiveBeginPlay`
  (set `self.BaseSpeed` (`CharacterMovementComponent.MaxWalkSpeed` (`self.CharacterMovement`)))
  (`self.SetSpeed`)
  (`self.SetStrength`))

(event `/Game/TimeGauntlet/BPI_Age.AgeUp`
  (params (AgeUp :type Boolean))
  (bind _current_age (`self.Current Age`))
  (bind _current_age_2 (`self.Current Age`))
  (bind _current_age_3 (`self.Current Age`))
  ;[1 1 1] Changes age
  (if AgeUp
    (if (not (>= _current_age_3 80.0))
      (set `self.Current Age` (+ _current_age 1.0))
      (`self.SetSpeed` :!label _label)
      (`KismetSystemLibrary.PrintString` (`KismetStringLibrary.Conv_DoubleToString` (`self.Current Age`)))
      (`self.UpdateTexture`)
      (if (or (== _current_age_2 0.0) (== _current_age_2 (`self.Max Age`)))
        (`self.Death`)
        (`SceneComponent.SetVisibility` (`self.Cube`) false false)
        (`KismetSystemLibrary.Delay` 0.2)
        (`self.K2_DestroyActor`)))
    (elif (> _current_age_3 0.0)
      (set `self.Current Age` (- _current_age 1.0))
      (goto _label))))

(event `/Game/BPI_Damagable.Hit`
  (params (Damage :type "Float (double-precision)"))
  ;[1 1 1] Handles taking damage
  (bind _output_get (set `self.Health` (- (`self.Health`) (- Damage (+ (* (/ (`self.Current Age`) (`self.Max Age`)) (`self.MaxResistance`)) (`self.MinResistance`))))))
  (`KismetSystemLibrary.PrintString` (`KismetStringLibrary.Conv_DoubleToString` _output_get))
  (if (<= _output_get 0.0)
    (`self.Death`)))

(event `Death`
  (`KismetSystemLibrary.PrintString` (`KismetStringLibrary.Concat_StrStr` (`KismetSystemLibrary.GetObjectName` self) "Is Dead"))
  ;[1 1 1] Drops items on death (doesnt do anything yet, Item drop always empty)
  (if (not (== (`self.ItemDrop`) null))
    (`|SpawnActorFromClass` (`self.ItemDrop`) (`self.GetTransform` self) "Undefined" "OverrideRootScale" null null)))

(event `UpdateTexture`
  ;[1 1 1] Comment
  (`MeshComponent.SetScalarParameterValueOnMaterials` (`self.Cube`) "Opacity" (/ (`self.Current Age`) (`self.Max Age`)))
  (`self.SetStrength`))

(event `/Game/BPI_Damagable.Freeze`
  (`KismetSystemLibrary.PrintString` "Freeze hit"))

(event `Trigger Attack`)

(fn `SetSpeed`
  (set `CharacterMovementComponent.MaxWalkSpeed` (+ (* (- 1.0 (/ (`self.Current Age`) (`self.Max Age`))) (`self.MaxSpeed`)) (`self.MinSpeed`)) (`self.CharacterMovement`))
  (`self.UpdateTexture`))

(fn `SetStrength`
  (set `self.Strength` (+ (* (/ (`self.Current Age`) (`self.Max Age`)) (`self.MaxStrength`)) (`self.MinStrength`))))

(fn `UserConstructionScript`)