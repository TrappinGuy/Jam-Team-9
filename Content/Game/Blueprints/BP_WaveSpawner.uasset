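; Wave spawner that runs an escalating enemy wave every ten seconds from BeginPlay through a self-calling, delayed WaveTick.
; Each tick raises WaveScore, which SpawnWave spends as a budget on random cost keys from the EnemyWaves map.
; Random picks re-roll at each use, so checked, deducted and printed costs can differ.
; The SpawnActor step using random SpawnPoints boxes is disconnected, so waves only print costs.
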(event `self.ReceiveBeginPlay`
  (`self.WaveTick`))

(event `WaveTick`
  (set `self.WaveScore` (+ (`self.WaveScore`) (`self.WaveScoreIncrease`)))
  (`KismetSystemLibrary.Delay` 10.0)
  (`self.SpawnWave`)
  (`self.WaveTick`))

(event `SpawnWave`
  (bind _result (`/Engine/EditorBlueprintResources/StandardMacros.IncrementInt` (`self.WaveCounter`))
    (:`  `
      (set `self.WaveCounter` _result)
      ;[1 1 1] Manages how strong a wave is
      (bind _output_get (set `self.WaveScoreToUse` (`self.WaveScore`)))
      (while (> _output_get 0)
        ;[1 1 1] Spawns enemy waves
        ;;[1 1 1] Get an enemy wave to spawn
        (bind _keys (`BlueprintMapLibrary.Map_Keys` (`self.EnemyWaves`)))
        (bind _output (`|GetArrayItem` _keys (`KismetMathLibrary.RandomInteger` (`KismetArrayLibrary.Array_Length` _keys))))
        (if (<= _output (`self.WaveScoreToUse`))
          (set `self.WaveScoreToUse` (- (`self.WaveScoreToUse`) _output))
          (`KismetSystemLibrary.PrintString` (`KismetStringLibrary.Conv_IntToString` _output)))))))

(fn `UserConstructionScript`)