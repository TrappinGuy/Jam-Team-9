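; Player revolver that trails the owner's right hand with drift, faces the camera, and cycles four fire modes via nested FlipFlops.
; Regular (distance falloff) and Freeze hit BPI_Damagable actors by camera trace; Incendiary spawns an actor at the impact; Explosive launches a projectile.
; Modes spend different ammo, and insufficient ammo triggers a timed reload with UI.
; Shots shake the camera and snap meshes between recoil poses; traced shots add a mode-coloured Niagara laser.
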(event `self.ReceiveBeginPlay`
  (bind _returnvalue_location (`KismetMathLibrary.BreakTransform` (`SceneComponent.GetRelativeTransform` (`self.ProjectileSpawnpoint`))))
  (bind _returnvalue (`|CreateWidget` "/Game/Game/Revolver/Reloading_UI.Reloading_UI_C"))
  (`UserWidget.AddToViewport` _returnvalue 0)
  (bind _output_get (set `self.ReloadingDisplay` _returnvalue))
  (`Widget.SetVisibility` _output_get "Hidden")
  (`FXSystemComponent.SetVectorParameter` (`self.LaserEffect`) "LaserStart" _returnvalue_location))

(event `self.ReceiveTick`
  (params (DeltaSeconds :type "Float (single-precision)"))
  (bind _returnvalue (`self.GetTransform`))
  (bind _gun_drift (`self.Gun_Drift`))
  (bind (_returnvalue_x _returnvalue_y _returnvalue_z) (`KismetMathLibrary.BreakVector` (- (`SceneComponent.K2_GetComponentLocation` (`/Game/FirstPerson/Blueprints/BP_FirstPersonCharacter.Right Hand` (`self.Owner_Reference`))) (`KismetMathLibrary.MakeVector` (.x (.location _returnvalue)) (.y (.location _returnvalue)) (.z (.location _returnvalue))))))
  (`self.K2_SetActorTransform` (`KismetMathLibrary.MakeTransform` (`KismetMathLibrary.MakeVector` (+ (/ _returnvalue_x _gun_drift) (.x (.location _returnvalue))) (+ (/ _returnvalue_y _gun_drift) (.y (.location _returnvalue))) (+ (/ _returnvalue_z _gun_drift) (.z (.location _returnvalue)))) (`PlayerCameraManager.GetCameraRotation` (`GameplayStatics.GetPlayerCameraManager` 0)))))

(event `Reload`
  (if (not (`self.isReloading`))
    (`Widget.SetVisibility` (`self.ReloadingDisplay`) "Visible")
    (set `self.isReloading` true)
    (`KismetSystemLibrary.Delay` 1.0)
    (set `self.isReloading` false)
    (set `self.Current_Ammo` (`self.Max_Ammo`))
    (`Widget.SetVisibility` (`self.ReloadingDisplay`) "Hidden")))

(event `FireGun`
  (bind _revolver_chamber (`self.Revolver_Chamber`))
  (bind _revolver_chamber_2 (`self.Revolver_Chamber`))
  (bind _revolver_bullets (`self.Revolver_Bullets`))
  (bind _revolver_bullets_2 (`self.Revolver_Bullets`))
  (bind _revolver (`self.Revolver`))
  (bind _revolver_2 (`self.Revolver`))
  (bind _revolver_chamber_3 (`self.Revolver_Chamber`))
  (bind _revolver_chamber_4 (`self.Revolver_Chamber`))
  (bind _revolver_bullets_3 (`self.Revolver_Bullets`))
  (bind _revolver_bullets_4 (`self.Revolver_Bullets`))
  (bind _revolver_3 (`self.Revolver`))
  (bind _revolver_4 (`self.Revolver`))
  (bind (_returnvalue_location _returnvalue_rotation) (`KismetMathLibrary.BreakTransform` (`SceneComponent.GetRelativeTransform` (`self.Revolver_Chamber_move_to`))))
  (bind (_returnvalue_location_2 _returnvalue_rotation_2) (`KismetMathLibrary.BreakTransform` (`SceneComponent.GetRelativeTransform` (`self.Revolver_Chamber_base`))))
  (bind (_returnvalue_location_3 _returnvalue_rotation_3) (`KismetMathLibrary.BreakTransform` (`SceneComponent.GetRelativeTransform` (`self.Revolver_Bullets_move_to`))))
  (bind (_returnvalue_location_4 _returnvalue_rotation_4) (`KismetMathLibrary.BreakTransform` (`SceneComponent.GetRelativeTransform` (`self.Revolver_Bullets_base`))))
  (bind (_returnvalue_location_5 _returnvalue_rotation_5) (`KismetMathLibrary.BreakTransform` (`SceneComponent.GetRelativeTransform` (`self.Revolver_move_to`))))
  (bind (_returnvalue_location_6 _returnvalue_rotation_6) (`KismetMathLibrary.BreakTransform` (`SceneComponent.GetRelativeTransform` (`self.Revolver_base`))))
  (bind (_returnvalue_location_7 _returnvalue_rotation_7) (`KismetMathLibrary.BreakTransform` (`SceneComponent.GetRelativeTransform` (`self.Revolver_Chamber_move_to`))))
  (bind (_returnvalue_location_8 _returnvalue_rotation_8) (`KismetMathLibrary.BreakTransform` (`SceneComponent.GetRelativeTransform` (`self.Revolver_Chamber_base`))))
  (bind (_returnvalue_location_9 _returnvalue_rotation_9) (`KismetMathLibrary.BreakTransform` (`SceneComponent.GetRelativeTransform` (`self.Revolver_Bullets_move_to`))))
  (bind (_returnvalue_location_10 _returnvalue_rotation_10) (`KismetMathLibrary.BreakTransform` (`SceneComponent.GetRelativeTransform` (`self.Revolver_Bullets_base`))))
  (bind (_returnvalue_location_11 _returnvalue_rotation_11) (`KismetMathLibrary.BreakTransform` (`SceneComponent.GetRelativeTransform` (`self.Revolver_move_to`))))
  (bind (_returnvalue_location_12 _returnvalue_rotation_12) (`KismetMathLibrary.BreakTransform` (`SceneComponent.GetRelativeTransform` (`self.Revolver_base`))))
  (bind _rootcomponent (`Actor.RootComponent` (`GameplayStatics.GetPlayerCameraManager` 0)))
  (bind _rootcomponent_2 (`Actor.RootComponent` (`GameplayStatics.GetPlayerCameraManager` 0)))
  (bind _returnvalue (`SceneComponent.K2_GetComponentLocation` _rootcomponent_2))
  (if (`self.isReloading`)
    _
    (elif (> (`self.Current_Ammo`) 0)
      (switch `/Game/Game/Blueprints/ENUM_FireModes` (`self.FireMode`)
        (:`NewEnumerator0`
          (bind (_outhit _returnvalue_2) (`KismetSystemLibrary.LineTraceSingle` _returnvalue (+ (* (`KismetMathLibrary.GetForwardVector` (`SceneComponent.K2_GetComponentRotation` _rootcomponent_2)) 3000.0) _returnvalue) "TraceTypeQuery1" true :!label _label))
          (switch `/Game/Game/Blueprints/ENUM_FireModes` (`self.FireMode`)
            (:`NewEnumerator0`
              (`FXSystemComponent.SetColorParameter` (`self.LaserEffect`) "Colour" (struct :`R` 0.046875 :`G` 0.046875 :`B` 0.046875 :`A` 1.0)))
            (:`NewEnumerator2`
              (`FXSystemComponent.SetColorParameter` (`self.LaserEffect`) "Colour" (struct :`R` 0.5 :`G` 1.0 :`B` 5.0 :`A` 1.0)))
            (:`NewEnumerator3`
              (`FXSystemComponent.SetColorParameter` (`self.LaserEffect`) "Colour" (struct :`R` 1.0 :`A` 1.0))))
          (if _returnvalue_2
            (`FXSystemComponent.SetVectorParameter` (`self.LaserEffect`) "LaserEnd" (`.Location` (`GameplayStatics.BreakHitResult` _outhit)))
            (else
              (`FXSystemComponent.SetVectorParameter` (`self.LaserEffect`) "LaserEnd" (+ (* (`KismetMathLibrary.GetForwardVector` (`SceneComponent.K2_GetComponentRotation` _rootcomponent)) 3000.0) (`SceneComponent.K2_GetComponentLocation` _rootcomponent)))))
          (`NiagaraComponent.ResetSystem` (`self.LaserEffect`))
          (`AddComponent|NODE_AddNiagaraComponent-0` :`RelativeTransform` (`SceneComponent.GetRelativeTransform` (`self.ProjectileSpawnpoint`)))
          (if (`|EnumInequality` (`self.FireMode`) "NewEnumerator3")
            ;[1 1 1] Checks to see if hit something damagable, if it has looks at the type of damage
            (if (`KismetSystemLibrary.DoesImplementInterface` (`.HitActor` (`GameplayStatics.BreakHitResult` _outhit)) "/Game/BPI_Damagable.BPI_Damagable_C")
              (switch `/Game/Game/Blueprints/ENUM_FireModes` (`self.FireMode`)
                (:`NewEnumerator0`
                  (message `/Game/BPI_Damagable.Hit` (`.HitActor` (`GameplayStatics.BreakHitResult` _outhit)) (* (- 1.0 (`KismetMathLibrary.Square` (/ (`.Distance` (`GameplayStatics.BreakHitResult` _outhit)) (`self.Max_Range`)))) (`self.Max_Damage`))))
                (:`NewEnumerator2`
                  (message `/Game/BPI_Damagable.Freeze` (`.HitActor` (`GameplayStatics.BreakHitResult` _outhit))))))
            ;[1 1 1] Reduces ammo
            (set `self.Current_Ammo` (- (`self.Current_Ammo`) 1))
            (else
              (`|SpawnActorFromClass` "/Game/Game/Blueprints/BP_Incendiary.BP_Incendiary_C" (`KismetMathLibrary.Conv_VectorToTransform` (`.Location` (`GameplayStatics.BreakHitResult` _outhit))) "Undefined" "OverrideRootScale" null null)
              (set `self.Current_Ammo` (- (`self.Current_Ammo`) 3))))
          (set `self.is_recoiling` true :!label _label_2)
          (`GameplayStatics.PlayWorldCameraShake` "/Game/Game/Blueprints/BP_GunCamShake.BP_GunCamShake_C" (`self.K2_GetActorLocation` (`GameplayStatics.GetPlayerCharacter` 0)) 0.0 1000.0)
          (if (`self.is_recoiling`)
            (`SceneComponent.K2_SetRelativeLocation` _revolver_chamber_4 _returnvalue_location_7 false false)
            (`SceneComponent.K2_SetRelativeRotation` _revolver_chamber_4 _returnvalue_rotation_7 false false)
            (else
              (`SceneComponent.K2_SetRelativeLocation` _revolver_chamber_3 _returnvalue_location_8 false false)
              (`SceneComponent.K2_SetRelativeRotation` _revolver_chamber_3 _returnvalue_rotation_8 false false)))
          (if (`self.is_recoiling`)
            (`SceneComponent.K2_SetRelativeLocation` _revolver_bullets_4 _returnvalue_location_9 false false)
            (`SceneComponent.K2_SetRelativeRotation` _revolver_bullets_4 _returnvalue_rotation_9 false false)
            (else
              (`SceneComponent.K2_SetRelativeLocation` _revolver_bullets_3 _returnvalue_location_10 false false)
              (`SceneComponent.K2_SetRelativeRotation` _revolver_bullets_3 _returnvalue_rotation_10 false false)))
          (if (`self.is_recoiling`)
            (`SceneComponent.K2_SetRelativeLocation` _revolver_4 _returnvalue_location_11 false false)
            (`SceneComponent.K2_SetRelativeRotation` _revolver_4 _returnvalue_rotation_11 false false)
            (else
              (`SceneComponent.K2_SetRelativeLocation` _revolver_3 _returnvalue_location_12 false false)
              (`SceneComponent.K2_SetRelativeRotation` _revolver_3 _returnvalue_rotation_12 false false)))
          (`KismetSystemLibrary.RetriggerableDelay` 0.07)
          (set `self.is_recoiling` false)
          (if (`self.is_recoiling`)
            (`SceneComponent.K2_SetRelativeLocation` _revolver_chamber_2 _returnvalue_location false false)
            (`SceneComponent.K2_SetRelativeRotation` _revolver_chamber_2 _returnvalue_rotation false false)
            (else
              (`SceneComponent.K2_SetRelativeLocation` _revolver_chamber _returnvalue_location_2 false false)
              (`SceneComponent.K2_SetRelativeRotation` _revolver_chamber _returnvalue_rotation_2 false false)))
          (if (`self.is_recoiling`)
            (`SceneComponent.K2_SetRelativeLocation` _revolver_bullets_2 _returnvalue_location_3 false false)
            (`SceneComponent.K2_SetRelativeRotation` _revolver_bullets_2 _returnvalue_rotation_3 false false)
            (else
              (`SceneComponent.K2_SetRelativeLocation` _revolver_bullets _returnvalue_location_4 false false)
              (`SceneComponent.K2_SetRelativeRotation` _revolver_bullets _returnvalue_rotation_4 false false)))
          (if (`self.is_recoiling`)
            (`SceneComponent.K2_SetRelativeLocation` _revolver_2 _returnvalue_location_5 false false)
            (`SceneComponent.K2_SetRelativeRotation` _revolver_2 _returnvalue_rotation_5 false false)
            (else
              (`SceneComponent.K2_SetRelativeLocation` _revolver _returnvalue_location_6 false false)
              (`SceneComponent.K2_SetRelativeRotation` _revolver _returnvalue_rotation_6 false false))))
        (:`NewEnumerator1`
          (if (> (`self.Current_Ammo`) 5)
            (`|SpawnActorFromClass` "/Game/FirstPerson/Blueprints/BP_ExplosiveProjectile.BP_ExplosiveProjectile_C" (`SceneComponent.K2_GetComponentToWorld` (`self.ProjectileSpawnpoint`)) "Undefined" "OverrideRootScale" null null)
            (set `self.Current_Ammo` 0)
            (goto _label_2)
            (else
              (`self.Reload`))))
        (:`NewEnumerator2`
          (goto _label))
        (:`NewEnumerator3`
          (if (> (`self.Current_Ammo`) 2)
            (goto _label)
            (else
              (`self.Reload`)))))
      (else
        (`self.Reload`)))))

(event `SwapFireType`
  (bind _revolver_bullets (`self.Revolver_Bullets`))
  ;[1 1 1] Change what projectile is fired
  (`/Engine/EditorBlueprintResources/StandardMacros.FlipFlop`
    (:`A`
      (`/Engine/EditorBlueprintResources/StandardMacros.FlipFlop`
        (:`A`
          (set `self.FireMode` "NewEnumerator1")
          (`PrimitiveComponent.SetMaterial` _revolver_bullets 0 "/Game/Game/Revolver/ExplodeBullets.ExplodeBullets"))
        (:`B`
          (set `self.FireMode` "NewEnumerator3")
          (`PrimitiveComponent.SetMaterial` _revolver_bullets 0 "/Game/Game/Revolver/IncBullets.IncBullets"))))
    (:`B`
      (`/Engine/EditorBlueprintResources/StandardMacros.FlipFlop`
        (:`A`
          (set `self.FireMode` "NewEnumerator2")
          (`PrimitiveComponent.SetMaterial` _revolver_bullets 0 "/Game/Game/Revolver/FreezeBullets.FreezeBullets"))
        (:`B`
          (set `self.FireMode` "NewEnumerator0")
          (`PrimitiveComponent.SetMaterial` _revolver_bullets 0 "/Game/Game/Revolver/RegBullets.RegBullets"))))))

(fn `UserConstructionScript`)