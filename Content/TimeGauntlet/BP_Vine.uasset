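; BP_Vine is an actor in TimeGauntlet whose Sphere component fades in or out as it is aged up or down.
; SnapAge takes an AgeUp flag and uses the Aged state to ignore repeated requests in the same direction.
; A change toggles the sphere's shadow casting and plays or reverses the Phase timeline, which drives the Opacity parameter on its materials.
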(event `/Game/TimeGauntlet/BPI_AgeSnap.SnapAge`
  (params (AgeUp :type Boolean))
  (bind _aged_ (`self.Aged?`))
  (bind _sphere (`self.Sphere`))
  ;[1 1 1] Checks if it is aging up or down
  (if AgeUp
    (if (not _aged_)
      (`PrimitiveComponent.SetCastShadow` _sphere true)
      (set `self.Aged?` true)
      ;[1 1 1] Phases sphere in and out of visibility
      (bind (_direction _newtrack_0) (`Timeline|Phase` :!label _label)
        (:`Update`
          (`MeshComponent.SetScalarParameterValueOnMaterials` (`self.Sphere`) "Opacity" _newtrack_0))))
    (elif _aged_
      (`PrimitiveComponent.SetCastShadow` _sphere false)
      (set `self.Aged?` false)
      (goto _label :!via `Reverse`))))

(fn `UserConstructionScript`)